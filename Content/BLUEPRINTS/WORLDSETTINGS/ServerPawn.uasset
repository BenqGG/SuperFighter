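; Server-side view pawn that follows one or two SPPawnBP players along the X/Z plane and reclaims the view target whenever it loses it.
; On authority, Tick rescans for players until two are valid, then calls SetPos.
; SetPos tracks a lone player at fixed depth, or centers between two, pulling back along Y as their X separation grows.
; A HitTest debug input triggers LightAttack on the first player pawn found.
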(event EventBeginPlay
  ;[1 1 1] BEGIN PLAY
  (Networking|SwitchHasAuthority
    (:Authority
      (Variables|Default|SetPlayersAmount 0)
      (Class|PlayerController|ActivateTouchInterface (Game|GetPlayerController 0)))))

(event Collision|EventActorBeginOverlap
  (params (OtherActor :type Actor%20Object%20Reference)))

(event EventTick
  (params (DeltaSeconds :type Float%20%28single-precision%29))
  (bind _player1 (Variables|Default|GetPlayer1))
  ;[1 1 1] TICK
  (Networking|SwitchHasAuthority
    (:Authority
      (if (and (Utilities|IsValid (Utilities|Array|Get(acopy) _player1)) (Utilities|IsValid (Utilities|Array|Get(acopy) _player1 1)))
        (CallFunction|SetPos)
        (else
          (bind _outactors (Actor|GetAllActorsOfClass "/Game/BLUEPRINTS/WORLDSETTINGS/SPPawnBP.SPPawnBP_C"))
          (Utilities|Array|Clear (Variables|Default|GetPlayer1))
          (for _array_element _outactors
            (Utilities|Array|AddUnique (Variables|Default|GetPlayer1) _array_element))
          (Variables|Default|SetPlayersAmount (Utilities|Array|Length (Variables|Default|GetPlayer1)))
          (CallFunction|SetPos))))))

(event EventOnEndViewTarget
  (params (PC :type Player%20Controller%20Object%20Reference))
  ;[1 1 1] END VIEW TARGET
  (Networking|SwitchHasAuthority
    (:Authority
      (Game|Player|SetViewTargetwithBlend PC self 0.0 "VTBlend_Linear" 0.0 false))))

(event Input|ActionEvents|InputActionHitTest
  (params (Key :type Key%20Structure :default "AnyKey"))
  ;[1 1 1] TEST KEY
  (:Pressed
    (Development|PrintString "Server Attack")
    (Networking|SwitchHasAuthority
      (:Authority
        (bind _outactors (Actor|GetAllActorsOfClass "/Game/BLUEPRINTS/WORLDSETTINGS/SPPawnBP.SPPawnBP_C"))
        (Class|SPPawnCPP|LightAttack (Utilities|Array|Get(acopy) _outactors) 1)))))

(fn ConstructionScript)

(fn SetPos
  (bind _player1 (Variables|Default|GetPlayer1))
  (bind _player1_2 (Variables|Default|GetPlayer1))
  (bind _item (Utilities|Array|Get(acopy) _player1_2))
  (bind _item_2 (Utilities|Array|Get(acopy) _player1_2 1))
  (bind _item_3 (Utilities|Array|Get(acopy) _player1))
  (bind _returnvalue (Transformation|GetActorLocation _item_3))
  (bind _returnvalue_2 (Transformation|GetActorLocation _item))
  (bind _returnvalue_3 (Transformation|GetActorLocation _item_2))
  (bind (_x _y _z) (Math|Vector|BreakVector _returnvalue))
  (bind (_x_2 _y_2 _z_2) (Math|Vector|BreakVector _returnvalue_2))
  (bind (_x_3 _y_3 _z_3) (Math|Vector|BreakVector _returnvalue_3))
  (if (== (Variables|Default|GetPlayersAmount) 1)
    (Transformation|SetActorLocation (Math|Vector|MakeVector _x 8e+02 _z) false false)
    (elif (== (Variables|Default|GetPlayersAmount) 2)
      (LocalVariables|SetMiddleX (+ (/ (- _x_2 _x_3) 2.0) _x_3))
      (LocalVariables|SetMiddleY (+ _z_3 (/ (- _z_2 _z_3) 2.0)))
      (LocalVariables|SetMiddleZoom (+ (/ (Math|Float|Absolute(Float) (- _x_2 _x_3)) 2.0) 3e+02))
      (Transformation|SetActorLocation (Math|Vector|MakeVector (LocalVariables|GetMiddleX) (LocalVariables|GetMiddleZoom) (LocalVariables|GetMiddleY)) false false))))