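; Player controller Blueprint that sets up the local HUD and touch controls and provides pawn spawning.
; BeginPlay creates the SPMainHUD widget and activates a left-only virtual joystick on player controller 0.
; NativeSpawnSPPawnBP spawns SomaCruz at a given location on authority only, ignoring its Server flag; the server couch pawn spawn is unconnected.
; AxisPosition packs two input axis key values into a 2D vector.
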(event EventBeginPlay
  (bind _returnvalue (Game|GetPlayerController 0))
  (Networking|SwitchHasAuthority
    (:Authority
      _)
    (:Remote
      _))
  (bind _returnvalue_2 (UserInterface|CreateWidget "/Game/BLUEPRINTS/HUD/SPMainHUD.SPMainHUD_C" _returnvalue))
  (UserInterface|Viewport|AddtoViewport _returnvalue_2 0)
  (Class|PlayerController|ActivateTouchInterface _returnvalue "/Game/BLUEPRINTS/HUD/PlayerControll/LeftVirtualJoystickOnly.LeftVirtualJoystickOnly"))

(event EventTick
  (params (DeltaSeconds :type Float%20%28single-precision%29)))

(fn ConstructionScript)

(fn NativeSpawnSPPawnBP
  (params (Location :type Vector) (Server :type Boolean))
  (Networking|SwitchHasAuthority
    (:Authority
      (if Server
        _
        (else
          _))
      (bind _returnvalue (Game|SpawnActorfromClass "/Game/BLUEPRINTS/WORLDSETTINGS/SomaCruz.SomaCruz_C" (Math|Conversions|ToTransform(Vector) Location) "AlwaysSpawn" 0 0))
      (return _returnvalue))
    (:Remote
      (return 0))))

(fn AxisPosition
  (return (Math|Vector2D|MakeVector2D (Class|Actor|GetInputAxisKeyValue) (Class|Actor|GetInputAxisKeyValue))))