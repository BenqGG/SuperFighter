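; SPGameInstanceBP is a Game Instance Blueprint that handles network failures and online session cleanup.
; On a lost connection it destroys the session and opens the MainMenu level whether that succeeds or fails.
; A connection timeout only prints a debug string.
; On shutdown it calls the parent implementation, then destroys the session.
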(event EventHandleNetworkError
  (params (FailureType :type ENetworkFailure%20Enum :default "NetDriverAlreadyExists") (bIsServer :type Boolean))
  ;[1 1 1] NETWORK ERROR
  (switch Utilities|FlowControl|Switch|SwitchonENetworkFailure FailureType
    (:ConnectionLost
      (Development|PrintString "LOST")
      (|DestroySession (Game|GetPlayerController 0)
        (:then
          (Development|PrintString "Exiting ..."))
        (:OnSuccess
          (Development|PrintString "Exit Succes")
          (Game|OpenLevel(byName) "MainMenu" :!label _label))
        (:OnFailure
          (Development|PrintString "Exit Failure")
          (goto _label))))
    (:ConnectionTimeout
      (Development|PrintString "TMIE OUT"))))

(event EventShutdown
  ;[1 1 1] SHUT DOWN
  (|CallParentFunction)
  (|DestroySession (Game|GetPlayerController 0)))