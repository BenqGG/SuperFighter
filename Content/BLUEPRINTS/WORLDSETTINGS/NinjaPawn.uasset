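; NinjaPawn is a side-view fighter character with movement, jump, defence, dash, spot dodge and a two-hit light attack.
; Actions form a delegate-driven state machine: each resets timing and permissions, rebinds follow-up events and switches looping or one-shot animations.
; Attacks add force and spawn facing-aware SPHitBoxBP actors that follow the pawn.
; The server sets attributes, debug shapes show defence and stun, and hit-reaction functions are empty override stubs.
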(event Custom|MoveDelegate
  ;[1 1 1] Client Delegates Unnessesery for now
  (Networking|SwitchHasAuthority
    (:Remote
      (Development|PrintString "moving"))))

(event Custom|RunDelegate
  ;[1 1 1] Client Delegates Unnessesery for now
  (Networking|SwitchHasAuthority
    (:Remote
      (Development|PrintString "runing"))))

(event Custom|StopStrongAttackDelegate
  ;[1 1 1] Client Delegates Unnessesery for now
  (Networking|SwitchHasAuthority
    (:Remote
      (Class|SPPawnCPP|SetSAttackKey false))))

(event Custom|JumpDelegate
  ;[1 1 1] Client Delegates Unnessesery for now
  (Networking|SwitchHasAuthority
    (:Remote
      (Class|SPPawnCPP|SetJumpKey true))))

(event Custom|TouchGroundDelegate
  ;[1 1 1] Client Delegates Unnessesery for now
  (Networking|SwitchHasAuthority
    (:Remote
      (Development|PrintString "TouchGround"))))

(event Custom|Call%20Get%20Hit%20Action
  ;[1 1 1] CALL GET HIT
  (Actions|GetHitAction))

(event Custom|LeaveGroundDelegate
  ;[1 1 1] Client Delegates Unnessesery for now
  (Networking|SwitchHasAuthority
    (:Remote
      (Development|PrintString "Leave Ground"))))

(event Custom|StopJumpDelegate
  ;[1 1 1] Client Delegates Unnessesery for now
  (Networking|SwitchHasAuthority
    (:Remote
      (Class|SPPawnCPP|SetJumpKey false))))

(event Custom|StrongAttackDelegate
  ;[1 1 1] Client Delegates Unnessesery for now
  (Networking|SwitchHasAuthority
    (:Remote
      (Class|SPPawnCPP|SetSAttackKey true))))

(event Custom|StopMoveDelegate
  ;[1 1 1] Client Delegates Unnessesery for now
  (Networking|SwitchHasAuthority
    (:Remote
      (Development|PrintString "stop moving"))))

(event EventBeginPlay
  ;[1 1 1] BEGIN PLAY
  (|CallParentFunction)
  (Transformation|SetActorScale3D "0.200000,0.200000,0.200000"))

(event EventDrawDefence
  (bind _returnvalue (Transformation|GetActorLocation))
  (bind (_x _y _z) (Math|Vector|BreakVector _returnvalue))
  ;[1 1 1] DRAW DEFENCE
  (bind _newparam (SuperFighter|DefenceCircleRadius))
  (Rendering|Debug|DrawDebugCircle (Math|Vector|MakeVector _x _y (+ _z 2e+01)) _newparam 24 "(R=0.053687,G=0.000000,B=1.000000,A=1.000000)" 0.0 0.0 "1.000000,0.000000,0.000000" "0.000000,0.000000,1.000000"))

(event EventEndStun
  ;[1 1 1] END STUN
  (|CallParentFunction)
  (Actions|EndStunAction))

(event EventDrawStunMeter
  (params (Radius :type Float%20%28single-precision%29))
  (bind _returnvalue (Transformation|GetActorLocation))
  (bind (_x _y _z) (Math|Vector|BreakVector _returnvalue))
  ;[1 1 1] DRAW STUN METER
  (if (> Radius 0.0)
    (Rendering|Debug|DrawDebugBox (Math|Vector|MakeVector _x _y (+ _z 5e+01)) (Math|Vector|MakeVector Radius 1.0 2.0) "(R=1.000000,G=1.000000,B=1.000000,A=1.000000)" "0, 0, 0" 0.0 5.0)))

(event EventOnEndViewTarget
  (params (PC :type Player%20Controller%20Object%20Reference))
  ;[1 1 1] END VIEW
  (|CallParentFunction PC)
  (Networking|SwitchHasAuthority
    (:Authority
      (Class|SPPawnCPP|CallEndViewTarget))))

(event EventTick
  (params (DeltaSeconds :type Float%20%28single-precision%29)))

(event EventSetUpIdle
  ;[1 1 1] SET UP IDLE
  (SuperFighter|SetupIdleBP))

(event EventGetHit
  (params (hitstun :type Float%20%28single-precision%29) (damage :type Float%20%28single-precision%29) (knockback :type Vector))
  ;[1 1 1] GET HIT
  (|CallParentFunction hitstun damage knockback)
  (CallFunction|CallGetHitAction))

(event EventDashEnd
  ;[1 1 1] Dash End
  (Actions|DashEndAction))

(fn ConstructionScript)

(fn ScreentoGameCoords
  (params (NewParam :type Vector%202D%20Structure))
  (bind _returnvalue (Viewport|GetViewportSize))
  (bind (_x _y) (Math|Vector2D|BreakVector2D _returnvalue))
  (LocalVariables|SetScreenCoords NewParam)
  (LocalVariables|SetAspect (/ _x _y))
  (bind _output_get (LocalVariables|SetXHalfGameView (.Y (Math|Vector|BreakVector (Variables|/Script/Engine.SceneComponent|GetRelativeLocation (Variables|Default|GetCamera))))))
  (LocalVariables|SetLeftGameBorder (- (.X (Math|Vector|BreakVector (Transformation|GetActorLocation))) _output_get))
  (bind _output_get_2 (LocalVariables|SetScale (/ (.X (Math|Vector2D|BreakVector2D (Viewport|GetViewportSize))) (* (LocalVariables|GetXHalfGameView) 2.0))))
  (bind _output_get_3 (LocalVariables|Setx (/ (.X (Math|Vector2D|BreakVector2D (LocalVariables|GetScreenCoords))) _output_get_2)))
  (LocalVariables|SetDestX (+ _output_get_3 (LocalVariables|GetLeftGameBorder)))
  (LocalVariables|SetYHalfGameView (/ (LocalVariables|GetXHalfGameView) (LocalVariables|GetAspect)))
  (LocalVariables|SetTopGameBorder (+ (.Z (Math|Vector|BreakVector (Transformation|GetActorLocation))) (LocalVariables|GetYHalfGameView)))
  (bind _output_get_4 (LocalVariables|SetScale (/ (.Y (Math|Vector2D|BreakVector2D (Viewport|GetViewportSize))) (* (LocalVariables|GetYHalfGameView) 2.0))))
  (bind _output_get_5 (LocalVariables|Setx (/ (.Y (Math|Vector2D|BreakVector2D (LocalVariables|GetScreenCoords))) _output_get_4)))
  (LocalVariables|SetDestZ (- (LocalVariables|GetTopGameBorder) _output_get_5))
  (Development|PrintString (Utilities|String|ToString(Float) (- (LocalVariables|GetTopGameBorder) _output_get_5)))
  (return (Math|Vector|MakeVector (LocalVariables|GetDestX) 0.0 (LocalVariables|GetDestZ))))

(fn GroundUnderFeet
  (bind _collision_box (Variables|Default|Getcollision_box))
  (bind (_origin _boxextent) (Collision|GetComponentBounds _collision_box))
  (bind (_x _y _z) (Math|Vector|BreakVector _origin))
  (bind (_x_2 _y_2 _z_2) (Math|Vector|BreakVector _boxextent))
  (bind _returnvalue (- _z _z_2))
  (bind _returnvalue_2 (+ _x _x_2))
  (bind _returnvalue_3 (- _returnvalue 1.0))
  (bind _returnvalue_4 (Math|Vector|MakeVector _returnvalue_2 _y _returnvalue_3))
  (bind (_x_3 _y_3 _z_3) (Math|Vector|BreakVector _returnvalue_4))
  (bind _returnvalue_5 (Collision|LineTraceForObjects _returnvalue_4 (Math|Vector|MakeVector (- _x_3 (* _x_2 2.0)) _y_3 _z_3) (Utilities|Array|MakeArray "ObjectTypeQuery1") false 0 "None"))
  (return _returnvalue_5))

(fn GroundNexttoFeet
  (params (right :type Boolean))
  (bind _collision_box (Variables|Default|Getcollision_box))
  (bind _collision_box_2 (Variables|Default|Getcollision_box))
  (bind (_origin _boxextent) (Collision|GetComponentBounds _collision_box_2))
  (bind (_origin_2 _boxextent_2) (Collision|GetComponentBounds _collision_box))
  (bind (_x _y _z) (Math|Vector|BreakVector _origin))
  (bind (_x_2 _y_2 _z_2) (Math|Vector|BreakVector _boxextent))
  (bind (_x_3 _y_3 _z_3) (Math|Vector|BreakVector _origin_2))
  (bind (_x_4 _y_4 _z_4) (Math|Vector|BreakVector _boxextent_2))
  (bind _returnvalue (- _x _x_2))
  (bind _returnvalue_2 (+ _x_3 _x_4 2.0))
  (bind _returnvalue_3 (Math|Vector|MakeVector _returnvalue_2 _y_3 _z_3))
  (bind _returnvalue_4 (- _returnvalue 2.0))
  (bind _returnvalue_5 (Math|Vector|MakeVector _returnvalue_4 _y _z))
  (bind (_x_5 _y_5 _z_5) (Math|Vector|BreakVector _returnvalue_3))
  (bind (_x_6 _y_6 _z_6) (Math|Vector|BreakVector _returnvalue_5))
  (if right
    (LocalVariables|SetStart _returnvalue_3)
    (LocalVariables|SetEnd (Math|Vector|MakeVector _x_5 _y_5 (- _z_5 _z_4)))
    (else
      (LocalVariables|SetStart _returnvalue_5)
      (LocalVariables|SetEnd (Math|Vector|MakeVector _x_6 _y_6 (- _z_6 _z_2)))))
  (bind _returnvalue_6 (Collision|LineTraceForObjects (LocalVariables|GetStart) (LocalVariables|GetEnd) (Utilities|Array|MakeArray "ObjectTypeQuery1") false 0 "None"))
  (return _returnvalue_6))

(fn AxisPosition
  (bind _asspplayer_controller_bp (Utilities|Casting|CastToSPPlayerControllerBP (Game|GetPlayerController 0))
    (:then
      (bind _returnvalue (Class|SPPlayerControllerCPP|AxisPosition _asspplayer_controller_bp))
      (return _returnvalue))
    (:CastFailed
      (return ""))))

(fn SetStartupActions
  (Class|SPPawnCPP|StartNewAction)
  (Class|SPPawnCPP|ResetActions 0.0)
  (Animations|ResetAnimation)
  (Class|SPPawnCPP|SetCanMove true)
  (Class|SPPawnCPP|SetCanJump true)
  (Class|SPPawnCPP|SetCanDefence true)
  (Class|SPPawnCPP|SetCanDash true)
  (Class|SPPawnCPP|SetCanLightAttack true)
  (Variables|Default|SetActionSpotDodge (EventDispatchers|CreateEvent :!event SpotDodgeAction))
  (Variables|Default|SetActionDash (EventDispatchers|CreateEvent :!event DashAction))
  (Variables|Default|SetActionAirDash (EventDispatchers|CreateEvent :!event DashAction))
  (Variables|Default|SetActionMove (EventDispatchers|CreateEvent :!event MoveAction))
  (Variables|Default|SetActionTouchGround (EventDispatchers|CreateEvent :!event TouchGroundAction))
  (Variables|Default|SetActionLeaveGround (EventDispatchers|CreateEvent :!event LeaveGroundAction))
  (Variables|Default|SetActionJump (EventDispatchers|CreateEvent :!event JumpAction))
  (Variables|Default|SetActionYDirectionChange (EventDispatchers|CreateEvent :!event ResetAnimation))
  (Variables|Default|SetActionDefence (EventDispatchers|CreateEvent :!event DefenceAction))
  (Variables|Default|SetActionReleaseDefence (EventDispatchers|CreateEvent :!event ReleaseDefenceAction))
  (Variables|Default|SetActionLightAttack (EventDispatchers|CreateEvent :!event LightAttackAction)))

(fn Void)

(fn DefenceCircleRadius
  (bind _returnvalue (Class|SPPawnCPP|CurrentDefence))
  (return (/ (* _returnvalue 6e+01) (.Defence (Utilities|Struct|BreakSPPawnAttributes (Variables|Default|GetAttributes))))))

(fn DashEndAction
  (Actions|SetStartupActions))

(fn GetHitAction)

(fn EndStunAction)

(fn SetupIdleBP
  (Networking|SwitchHasAuthority
    (:Authority
      (Class|SPPawnCPP|SetAttributes (Utilities|Struct|MakeSPPawnAttributes (Variables|Default|GetMoveSpeed) 4e+02 2 1.6e+03 2e+02 1.5e+03 2e+01 1e+02 7.5e+02 0.2 0.3 0.4)))
    (:Remote
      _))
  (Class|SPPawnCPP|ResetRestrictions)
  (Actions|SetStartupActions)
  (Animations|ResetAnimation))

(fn ResetAnimation
  (bind _states (Variables|Default|GetStates))
  (bind (_move_right _move_left _jump _jump_left_wall _jump_right_wall _on_ground) (Utilities|Struct|BreakSPPawnStates _states))
  (if (Math|Boolean|ORBoolean (not _on_ground) _jump _jump_left_wall _jump_right_wall)
    (if (Math|Boolean|ORBoolean (>= (.Y (Math|Vector2D|BreakVector2D (Variables|Default|GetForces))) 0.0) _jump _jump_left_wall _jump_right_wall)
      (Animations|RiseAnimation)
      (else
        (Animations|FallAnimation)))
    (elif (or _move_right _move_left)
      (Animations|MoveAnimation)
      (else
        (Animations|IdleAnimation)))))

(fn IdleAnimation
  (Class|SPPawnCPP|ChangeAnimation (Utilities|Array|Get(acopy) (Variables|Default|GetAnimations)))
  (Components|Timeline|SetLooping (Variables|Default|Getanimation) true))

(fn MoveAction
  (Class|SPPawnCPP|ChangeMovementSpeed (Variables|Default|GetMoveSpeed))
  (Class|SPPawnCPP|StartNewAction)
  (Class|SPPawnCPP|ResetActions 0.5)
  (Class|SPPawnCPP|SetCanJump true)
  (Class|SPPawnCPP|SetCanDash true)
  (Class|SPPawnCPP|SetCanLightAttack true)
  (Variables|Default|SetActionJump (EventDispatchers|CreateEvent :!event JumpAction))
  (Variables|Default|SetActionStopMove (EventDispatchers|CreateEvent :!event SetStartupActions))
  (Variables|Default|SetActionDelay (EventDispatchers|CreateEvent :!event RunAction))
  (Variables|Default|SetActionLightAttack (EventDispatchers|CreateEvent :!event LightAttackAction))
  (Animations|MoveAnimation))

(fn MoveAnimation
  (if (CallFunction|GroundUnderFeet)
    (Class|SPPawnCPP|ChangeAnimation (Utilities|Array|Get(acopy) (Variables|Default|GetAnimations) 1))
    (Components|Timeline|SetLooping (Variables|Default|Getanimation) true)))

(fn RunAction
  (Class|SPPawnCPP|ResetActions 0.0)
  (Class|SPPawnCPP|ChangeMovementSpeed (Variables|Default|GetRunSpeed))
  (Animations|RunAnimation))

(fn RunAnimation
  (if (CallFunction|GroundUnderFeet)
    (Class|SPPawnCPP|ChangeAnimation (Utilities|Array|Get(acopy) (Variables|Default|GetAnimations) 2))
    (Components|Timeline|SetLooping (Variables|Default|Getanimation) true)))

(fn FallAnimation
  (Class|SPPawnCPP|ChangeAnimation (Utilities|Array|Get(acopy) (Variables|Default|GetAnimations) 3))
  (Components|Timeline|SetLooping (Variables|Default|Getanimation) true))

(fn TouchGroundAction
  (bind _states (Variables|Default|GetStates))
  (bind (_move_right _move_left) (Utilities|Struct|BreakSPPawnStates _states))
  (if (or _move_right _move_left)
    (if (== (.MoveSpeed (Utilities|Struct|BreakSPPawnAttributes (Variables|Default|GetAttributes))) (Variables|Default|GetMoveSpeed))
      (Actions|MoveAction)
      (else
        (Animations|RunAnimation)))
    (else
      (Animations|ResetAnimation))))

(fn LeaveGroundAction
  (if (not (.JUMP (Utilities|Struct|BreakSPPawnStates (Variables|Default|GetStates))))
    (Animations|ResetAnimation)))

(fn RiseAnimation
  (Class|SPPawnCPP|ChangeAnimation (Utilities|Array|Get(acopy) (Variables|Default|GetAnimations) 4))
  (Components|Timeline|SetLooping (Variables|Default|Getanimation) true))

(fn JumpAction
  (Class|SPPawnCPP|StartNewAction)
  (Class|SPPawnCPP|ResetActions 0.07)
  (Class|SPPawnCPP|SetCanMove true)
  (Class|SPPawnCPP|SetCanDash true)
  (Variables|Default|SetActionStopJump (EventDispatchers|CreateEvent :!event SetStartupActions))
  (Variables|Default|SetActionDelay (EventDispatchers|CreateEvent :!event StartJumpingAction))
  (Animations|JumpAnimation))

(fn JumpAnimation
  (bind _animation (Variables|Default|Getanimation))
  (Class|SPPawnCPP|ChangeAnimation (Utilities|Array|Get(acopy) (Variables|Default|GetAnimations) 5))
  (Components|Timeline|SetLooping _animation false)
  (EventDispatchers|BindEventtoOnFinishedPlaying _animation (EventDispatchers|CreateEvent :!event ResetAnimation)))

(fn StartJumpingAction
  (Class|SPPawnCPP|ResetActions 0.0)
  (Class|SPPawnCPP|StartJump))

(fn DefenceAction
  (Class|SPPawnCPP|StartNewAction)
  (Class|SPPawnCPP|ResetActions 0.0)
  (Animations|DefenceAnimation))

(fn ReleaseDefenceAction
  (Actions|SetStartupActions))

(fn DefenceAnimation
  (Class|SPPawnCPP|ChangeAnimation (Utilities|Array|Get(acopy) (Variables|Default|GetAnimations) 6))
  (Components|Timeline|SetLooping (Variables|Default|Getanimation) true))

(fn DashAction
  (Class|SPPawnCPP|StartNewAction)
  (Class|SPPawnCPP|ResetActions 0.0)
  (Animations|DashAnimation))

(fn DashAnimation
  (if (.SIDE_DASH (Utilities|Struct|BreakSPPawnStates (Variables|Default|GetStates)))
    (Class|SPPawnCPP|ChangeAnimation (Utilities|Array|Get(acopy) (Variables|Default|GetAnimations) 7))
    (Components|Timeline|SetLooping (Variables|Default|Getanimation) true)
    (else
      (Class|SPPawnCPP|ChangeAnimation (Utilities|Array|Get(acopy) (Variables|Default|GetAnimations) 8))
      (Components|Timeline|SetLooping (Variables|Default|Getanimation) true))))

(fn SpotDodgeAction
  (Class|SPPawnCPP|StartNewAction)
  (Class|SPPawnCPP|ResetActions 0.0)
  (Animations|SpotDodgeAnimation))

(fn SpotDodgeAnimation
  (Class|SPPawnCPP|ChangeAnimation (Utilities|Array|Get(acopy) (Variables|Default|GetAnimations) 7))
  (Components|Timeline|SetLooping (Variables|Default|Getanimation) true))

(fn LightAttackAction
  (Class|SPPawnCPP|StartNewAction)
  (Class|SPPawnCPP|ResetActions 0.17)
  (Class|SPPawnCPP|StartLightAttack 0.32)
  (Variables|Default|SetActionDelay (EventDispatchers|CreateEvent :!event LightAttackHitBoxAction))
  (Animations|LightAttack1Animation)
  (bind _returnvalue (Class|SPPawnCPP|FacingRight))
  (if _returnvalue
    (Class|SPPawnCPP|AddForce "1.000000,0.000000,200.000000")
    (else
      (Class|SPPawnCPP|AddForce "-1.000000,0.000000,200.000000"))))

(fn LightAttackHitBox
  (bind _returnvalue (Transformation|GetActorLocation))
  (bind (_x _y _z) (Math|Vector|BreakVector _returnvalue))
  (bind _returnvalue_2 (Game|SpawnActorfromClass "/Game/BLUEPRINTS/Physics/SPHitBoxBP.SPHitBoxBP_C" (Math|Transform|MakeTransform "0, 0, 0") "AlwaysSpawn" 0 0))
  (bind _returnvalue_3 (Class|SPPawnCPP|FacingRight))
  (if _returnvalue_3
    (LocalVariables|SetXModifier 3e+01)
    (LocalVariables|SetYModifier 33.8)
    (LocalVariables|SetForce "0.000000,1.000000,300.000000")
    (LocalVariables|SetTrajectory "0, 0, 0")
    (else
      (LocalVariables|SetXModifier -3e+01)
      (LocalVariables|SetYModifier 33.8)
      (LocalVariables|SetForce "0.000000,1.000000,300.000000")
      (LocalVariables|SetTrajectory "0.000000,0.000000,0.000000")))
  (LocalVariables|SetPosition (Math|Vector|MakeVector (+ (LocalVariables|GetXModifier) _x) (+ _z (LocalVariables|GetYModifier)) 15.0))
  (Class|SPHitBoxCPP|SetHitbox _returnvalue_2 (Utilities|Struct|MakeSPHitBoxDetails (LocalVariables|GetPosition) (LocalVariables|GetForce) 0.01 0.1 false false self 5.0 0.2 true (Math|Vector2D|MakeVector2D (LocalVariables|GetXModifier) (LocalVariables|GetYModifier)))))

(fn LightAttack1Animation
  (Class|SPPawnCPP|ChangeAnimation (Utilities|Array|Get(acopy) (Variables|Default|GetAnimations) 9))
  (Components|Timeline|SetLooping (Variables|Default|Getanimation) false))

(fn LightAttackAction2
  (Class|SPPawnCPP|StartNewAction)
  (Class|SPPawnCPP|ResetActions 0.1)
  (Class|SPPawnCPP|SetCanLightAttack true)
  (Variables|Default|SetActionDelay (EventDispatchers|CreateEvent :!event LightAttackAction3))
  (Variables|Default|SetActionLightAttack (EventDispatchers|CreateEvent :!event SecondLightAttackAction)))

(fn LightAttackAction3
  (Class|SPPawnCPP|StartNewAction)
  (Class|SPPawnCPP|ResetActions 0.05)
  (Variables|Default|SetActionDelay (EventDispatchers|CreateEvent :!event SetStartupActions)))

(fn SecondLightAttackAction
  (Class|SPPawnCPP|StartNewAction)
  (Class|SPPawnCPP|ResetActions 0.15)
  (Class|SPPawnCPP|StartLightAttack 0.3)
  (Variables|Default|SetActionDelay (EventDispatchers|CreateEvent :!event SecondLightAttackAction2))
  (Animations|LightAttack2Animation)
  (bind _returnvalue (Class|SPPawnCPP|FacingRight))
  (if _returnvalue
    (Class|SPPawnCPP|AddForce "1.000000,0.000000,100.000000")
    (else
      (Class|SPPawnCPP|AddForce "-1.000000,0.000000,100.000000"))))

(fn LightAttack2Animation
  (Class|SPPawnCPP|ChangeAnimation (Utilities|Array|Get(acopy) (Variables|Default|GetAnimations) 10))
  (Components|Timeline|SetLooping (Variables|Default|Getanimation) false))

(fn SecondLightAttackAction2
  (Class|SPPawnCPP|ResetActions 0.25)
  (HitBox|SecondLightAttackHitBox)
  (Variables|Default|SetActionDelay (EventDispatchers|CreateEvent :!event SetStartupActions)))

(fn LightAttackHitBoxAction
  (Class|SPPawnCPP|ResetActions 0.25)
  (HitBox|LightAttackHitBox)
  (Variables|Default|SetActionDelay (EventDispatchers|CreateEvent :!event LightAttackAction2)))

(fn SecondLightAttackHitBox
  (bind _returnvalue (Transformation|GetActorLocation))
  (bind (_x _y _z) (Math|Vector|BreakVector _returnvalue))
  (bind _returnvalue_2 (Game|SpawnActorfromClass "/Game/BLUEPRINTS/Physics/SPHitBoxBP.SPHitBoxBP_C" (Math|Transform|MakeTransform "0, 0, 0") "AlwaysSpawn" 0 0))
  (bind _returnvalue_3 (Class|SPPawnCPP|FacingRight))
  (if _returnvalue_3
    (LocalVariables|SetXModifier 4e+01)
    (LocalVariables|SetYModifier 25.0)
    (LocalVariables|SetForce "1.000000,0.000000,200.000000")
    (LocalVariables|SetTrajectory (LocalVariables|GetTrajectory))
    (else
      (LocalVariables|SetXModifier -4e+01)
      (LocalVariables|SetYModifier 25.0)
      (LocalVariables|SetForce "-1.000000,0.000000,200.000000")
      (LocalVariables|SetTrajectory "0.000000,0.000000,0.000000")))
  (LocalVariables|SetPosition (Math|Vector|MakeVector (+ (LocalVariables|GetXModifier) _x) (+ _z (LocalVariables|GetYModifier)) 15.0))
  (Class|SPHitBoxCPP|SetHitbox _returnvalue_2 (Utilities|Struct|MakeSPHitBoxDetails (LocalVariables|GetPosition) (LocalVariables|GetForce) 0.01 0.1 false false self 5.0 0.2 true (Math|Vector2D|MakeVector2D (LocalVariables|GetXModifier) (LocalVariables|GetYModifier)))))