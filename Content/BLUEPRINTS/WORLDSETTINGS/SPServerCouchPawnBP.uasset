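; Server couch pawn that tracks SomaCruz characters and provides test controls for driving one of them.
; FindPlayers extends the parent by packing every SomaCruz into SPSCPData, and ending a view target returns the player's view to this pawn on authority.
; Input actions forward attacks, jump, defence, dashes and spot dodge to the first SomaCruz found, on authority only.
; Walk input calls ServerMove on that character without an authority check.
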(event EventBeginPlay)

(event Collision|EventActorBeginOverlap
  (params (OtherActor :type Actor%20Object%20Reference)))

(event EventTick
  (params (DeltaSeconds :type Float%20%28single-precision%29)))

(event EventFindPlayers
  ;[1 1 1] FIND PLAYERS
  (|CallParentFunction)
  (bind _outactors (Actor|GetAllActorsOfClass "/Game/BLUEPRINTS/WORLDSETTINGS/SomaCruz.SomaCruz_C"))
  (Variables|Default|SetData (Utilities|Struct|MakeSPSCPData (Utilities|Array|Length _outactors) _outactors 1.5e+02)))

(event EventOnEndViewTarget
  (params (PC :type Player%20Controller%20Object%20Reference))
  ;[1 1 1] END VIEW TARGET
  (Networking|SwitchHasAuthority
    (:Authority
      (Game|Player|SetViewTargetwithBlend PC self 0.0 "VTBlend_Linear" 0.0 false))))

(event Input|ActionEvents|InputActionHitTest
  (params (Key :type Key%20Structure :default "AnyKey"))
  ;[1 1 1] LIGHT HIT TEST
  (:Pressed
    (Networking|SwitchHasAuthority
      (:Authority
        (bind _outactors (Actor|GetAllActorsOfClass "/Game/BLUEPRINTS/WORLDSETTINGS/SomaCruz.SomaCruz_C"))
        (Class|SPPawnCPP|LightAttack (Utilities|Array|Get(acopy) _outactors) 3)))))

(event Input|ActionEvents|InputActionJumpTest
  (params (Key :type Key%20Structure :default "AnyKey"))
  ;[1 1 1] JUMP TEST
  (:Pressed
    (Networking|SwitchHasAuthority
      (:Authority
        (bind _outactors (Actor|GetAllActorsOfClass "/Game/BLUEPRINTS/WORLDSETTINGS/SomaCruz.SomaCruz_C"))
        (Class|SPPawnCPP|Jump (Utilities|Array|Get(acopy) _outactors)))))
  (:Released
    (Networking|SwitchHasAuthority
      (:Authority
        (bind _outactors_2 (Actor|GetAllActorsOfClass "/Game/BLUEPRINTS/WORLDSETTINGS/SomaCruz.SomaCruz_C"))
        (Class|SPPawnCPP|StopJump (Utilities|Array|Get(acopy) _outactors_2))))))

(event Input|ActionEvents|InputActionWalkLeft
  (params (Key :type Key%20Structure :default "AnyKey"))
  ;[1 1 1] WALK
  (:Pressed
    (bind _outactors (Actor|GetAllActorsOfClass "/Game/BLUEPRINTS/WORLDSETTINGS/SomaCruz.SomaCruz_C"))
    (Class|SPPawnCPP|ServerMove (Utilities|Array|Get(acopy) _outactors) -1.0))
  (:Released
    (bind _outactors_2 (Actor|GetAllActorsOfClass "/Game/BLUEPRINTS/WORLDSETTINGS/SomaCruz.SomaCruz_C"))
    (Class|SPPawnCPP|ServerMove (Utilities|Array|Get(acopy) _outactors_2) 0.0)))

(event Input|ActionEvents|InputActionWalkRight
  (params (Key :type Key%20Structure :default "AnyKey"))
  ;[1 1 1] WALK
  (:Pressed
    (bind _outactors (Actor|GetAllActorsOfClass "/Game/BLUEPRINTS/WORLDSETTINGS/SomaCruz.SomaCruz_C"))
    (Class|SPPawnCPP|ServerMove (Utilities|Array|Get(acopy) _outactors) 1.0))
  (:Released
    (bind _outactors_2 (Actor|GetAllActorsOfClass "/Game/BLUEPRINTS/WORLDSETTINGS/SomaCruz.SomaCruz_C"))
    (Class|SPPawnCPP|ServerMove (Utilities|Array|Get(acopy) _outactors_2) 0.0)))

(event Input|ActionEvents|InputActionSideDash
  (params (Key :type Key%20Structure :default "AnyKey"))
  ;[1 1 1] SIDE DASH TEST
  (:Pressed
    (Networking|SwitchHasAuthority
      (:Authority
        (bind _outactors (Actor|GetAllActorsOfClass "/Game/BLUEPRINTS/WORLDSETTINGS/SomaCruz.SomaCruz_C"))
        (Class|SPPawnCPP|Defence (Utilities|Array|Get(acopy) _outactors) 2)))))

(event Input|ActionEvents|InputActionUpDash
  (params (Key :type Key%20Structure :default "AnyKey"))
  ;[1 1 1] UP DASH
  (:Pressed
    (Networking|SwitchHasAuthority
      (:Authority
        (bind _outactors (Actor|GetAllActorsOfClass "/Game/BLUEPRINTS/WORLDSETTINGS/SomaCruz.SomaCruz_C"))
        (Class|SPPawnCPP|Defence (Utilities|Array|Get(acopy) _outactors) 3)))))

(event Input|ActionEvents|InputActionStrongHitTest
  (params (Key :type Key%20Structure :default "AnyKey"))
  ;[1 1 1] STRONG HIT TEST
  (:Pressed
    (Networking|SwitchHasAuthority
      (:Authority
        (bind _outactors (Actor|GetAllActorsOfClass "/Game/BLUEPRINTS/WORLDSETTINGS/SomaCruz.SomaCruz_C"))
        (Class|SPPawnCPP|StrongAttack (Utilities|Array|Get(acopy) _outactors) 1))))
  (:Released
    (Networking|SwitchHasAuthority
      (:Authority
        (bind _outactors_2 (Actor|GetAllActorsOfClass "/Game/BLUEPRINTS/WORLDSETTINGS/SomaCruz.SomaCruz_C"))
        (Class|SPPawnCPP|ReleaseStrongAttack (Utilities|Array|Get(acopy) _outactors_2))))))

(event Input|ActionEvents|InputActionSpotDodge
  (params (Key :type Key%20Structure :default "AnyKey"))
  ;[1 1 1] SPOT DODGE
  (:Pressed
    (Networking|SwitchHasAuthority
      (:Authority
        (bind _outactors (Actor|GetAllActorsOfClass "/Game/BLUEPRINTS/WORLDSETTINGS/SomaCruz.SomaCruz_C"))
        (Class|SPPawnCPP|Defence (Utilities|Array|Get(acopy) _outactors) 4)))))

(event Input|ActionEvents|InputActionDefenceTest
  (params (Key :type Key%20Structure :default "AnyKey"))
  ;[1 1 1] DEFENCE TEST
  (:Pressed
    (Networking|SwitchHasAuthority
      (:Authority
        (bind _outactors (Actor|GetAllActorsOfClass "/Game/BLUEPRINTS/WORLDSETTINGS/SomaCruz.SomaCruz_C"))
        (Class|SPPawnCPP|Defence (Utilities|Array|Get(acopy) _outactors) 1))))
  (:Released
    (Networking|SwitchHasAuthority
      (:Authority
        (bind _outactors_2 (Actor|GetAllActorsOfClass "/Game/BLUEPRINTS/WORLDSETTINGS/SomaCruz.SomaCruz_C"))
        (Class|SPPawnCPP|ReleaseDefence (Utilities|Array|Get(acopy) _outactors_2))))))

(fn ConstructionScript)