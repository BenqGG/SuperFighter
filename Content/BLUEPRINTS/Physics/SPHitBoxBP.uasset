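; Hitbox actor that applies hitstun, damage and knockback to pawns it overlaps.
; On authority, an active hitbox calls GetHit on overlapped SPPawnCPP actors, skipping its owner unless friendly fire is enabled.
; Single-hit boxes destroy themselves after the first successful hit.
; Tick draws an authority-only debug circle at the sphere radius, red when active and green when inactive.
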(event EventBeginPlay)

(event Collision|EventActorBeginOverlap
  (params (OtherActor :type Actor%20Object%20Reference))
  (bind _details (Variables|Default|GetDetails))
  (bind (_position _force _activationtime _destroytime _friendlyfire _multihit _owner _damage _hitstun) (Utilities|Struct|BreakSPHitBoxDetails _details))
  ;[1 1 1] OVERLAP
  (Networking|SwitchHasAuthority
    (:Authority
      (if (Utilities|Struct|BreakSPHitBoxWorkData (Variables|Default|GetWorkData))
        (if (or _friendlyfire (!= _owner OtherActor))
          (bind _assppawn_cpp (Utilities|Casting|CastToSPPawnCPP OtherActor))
          (Class|SPPawnCPP|GetHit _assppawn_cpp _hitstun _damage _force)
          (if (not _multihit)
            (Class|SPHitBoxCPP|DestroyHitBox)))))))

(event EventTick
  (params (DeltaSeconds :type Float%20%28single-precision%29))
  (bind _returnvalue (Transformation|GetActorLocation))
  (bind _mainbody (Variables|Default|GetMainBody))
  (bind _sphereradius (Variables|/Script/Engine.SphereComponent|GetSphereRadius _mainbody))
  ;[1 1 1] TICK
  (Networking|SwitchHasAuthority
    (:Authority
      (if (Utilities|Struct|BreakSPHitBoxWorkData (Variables|Default|GetWorkData))
        (Rendering|Debug|DrawDebugCircle _returnvalue _sphereradius 45 "(R=1.000000,G=0.027806,B=0.000000,A=1.000000)" 0.0 0.0 "1.000000,0.000000,0.000000" "0.000000,0.000000,1.000000")
        (else
          (Rendering|Debug|DrawDebugCircle _returnvalue _sphereradius 45 "(R=0.000000,G=1.000000,B=0.136468,A=1.000000)" 0.0 0.0 "1.000000,0.000000,0.000000" "0.000000,0.000000,1.000000"))))))

(fn ConstructionScript)